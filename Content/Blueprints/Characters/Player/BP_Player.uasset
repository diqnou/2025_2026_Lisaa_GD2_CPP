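; BP_Player is the player Blueprint, linking its Health component to an on-screen HUD.
; On BeginPlay it creates WBP_HUD, seeds it with current and max health, then refreshes it whenever OnHealthChanged fires.
; A debug T key applies damage to itself through the Health component.
; An unconnected chain that would open a WBP_Calculette widget with UI-only input and a mouse cursor never runs.
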(event OnHealthChanged(Health)
  (params (NewHealth :type Float%20%28single-precision%29) (Delta :type Float%20%28single-precision%29))
  (Default|UpdateHealth (Variables|Widgets|HUD|GetHudWidgetRef) NewHealth (Variables|/Script/Lisaa.HealthComponent|GetMaxHealth (Variables|Default|GetHealth))))

(event EventBeginPlay
  (bind _health (Variables|Default|GetHealth))
  (bind _returnvalue (UserInterface|CreateWidget "/Game/Blueprints/Widgets/WBP_HUD.WBP_HUD_C")) ; CREATE WIDGET
  (bind _output_get (Variables|Widgets|HUD|SetHudWidgetRef _returnvalue))
  (Default|UpdateHealth _output_get (Class|HealthComponent|GetHealth _health) (Variables|/Script/Lisaa.HealthComponent|GetMaxHealth _health))
  (UserInterface|Viewport|AddtoViewport (Variables|Widgets|HUD|GetHudWidgetRef) 0))

(event Input|KeyboardEvents|DebugKeyT
  (params (Key :type Key%20Structure :default "None") (ActionValue :type Input%20Action%20Value%20Structure))
  (:Pressed
    (Class|HealthComponent|ApplyDamageat (Variables|Default|GetHealth) 5.0 self)))

(fn ConstructionScript)